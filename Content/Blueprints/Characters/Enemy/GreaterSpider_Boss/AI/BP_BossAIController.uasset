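; AI controller for the Greater Spider boss enemy, driving its behavior through a behavior tree.
; On BeginPlay it runs the spider boss behavior tree.
; Every tick it measures the distance between the controlled pawn and the first player character and writes it to the DistanceWithPlayer blackboard key for the tree to use.
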(event EventBeginPlay
  (AI|RunBehaviorTree "/Game/Blueprints/Characters/Enemy/GreaterSpider_Boss/AI/BT_SpiderEnemyBoss.BT_SpiderEnemyBoss"))

(event EventTick
  (params (DeltaSeconds :type Float%20%28single-precision%29))
  (AI|Components|Blackboard|SetValueasFloat (AI|GetBlackboard 0) (Utilities|Name|MakeLiteralName "DistanceWithPlayer") (Math|Vector|VectorLength (- (Transformation|GetActorLocation (Pawn|GetControlledPawn)) (Transformation|GetActorLocation (Game|GetPlayerCharacter 0))))))

(fn ConstructionScript)